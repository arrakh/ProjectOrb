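; Player character with camera-relative movement that fires and recalls a single energy orb and respawns enemies.
; Shoot press shows charge particles, and release launches the orb toward the camera trace's endpoint.
; Releasing again stops its projectile motion and runs a behavior tree to return it, where overlap destroys it.
; Enemy contact fades a HUD overlay and reloads M_Main; SpawnNewEnemy adds delayed replacements; the camera Lerp is unused.
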(event Custom|SpawnNewEnemy
  ;[1 1 1] SpawnNewEnemy() gets called from orb when enemy is hit
  (Utilities|FlowControl|Delay 5.0)
  (Game|SpawnActorfromClass "/Game/Blueprint/BP_Enemy.BP_Enemy_C" (Math|Transform|MakeTransform (.RandomLocation (AI|Navigation|GetRandomReachablePointinRadius (Math|Vector|MakeVector 0.0 0.0 0.0) 0.0 0 0)) "0, 0, 0" "2.000000,2.000000,2.000000") "AdjustIfPossibleButAlwaysSpawn" 0 0))

(event Collision|EventActorBeginOverlap
  (params (OtherActor :type Actor%20Object%20Reference))
  ;[1 1 1] Destroy orb when hitting player pawn
  (bind _asbp_energy_orb (Utilities|Casting|CastToBP_EnergyOrb OtherActor)
    (:then
      (if (Variables|Default|GetIsReturningOrb)
        (Actor|DestroyActor _asbp_energy_orb)
        (Variables|Default|SetIsReturningOrb false)
        (Variables|Default|SetHasOrbOut false)))
    (:CastFailed
      ;[1 1 1] Destroy us when hit by enemy
      (bind _asbp_enemy (Utilities|Casting|CastToBP_Enemy OtherActor))
      (Actor|DestroyActor _asbp_enemy)
      (bind _foundwidgets (Widget|GetAllWidgetsOfClass "/Game/Blueprint/WBP_HUD.WBP_HUD_C" true))
      (Widget|SetVisibility (Variables|/Game/Blueprint/WBP_HUD.WBP_HUD_C|GetImage_63 (Utilities|Array|Get(acopy) _foundwidgets)) "Visible") ; Redundant
      (Widget|SetVisibility (Variables|/Game/Blueprint/WBP_HUD.WBP_HUD_C|GetTextBlock_130 (Utilities|Array|Get(acopy) _foundwidgets)) "Visible")
      (Input|DisableInput 0)
      (bind _color (Timeline|TL_Death PlayFromStart)
        (:Update
          (Appearance|SetColorandOpacity (Variables|/Game/Blueprint/WBP_HUD.WBP_HUD_C|GetImage_63 (Utilities|Array|Get(acopy) _foundwidgets)) (Utilities|Struct|MakeLinearColor _color _color _color 1.0) :!class /Script/UMG.Image))
        (:Finished
          (Game|OpenLevel(byName) "M_Main"))))))

(event Input|ActionEvents|InputActionShoot
  (params (Key :type Key%20Structure))
  (bind _shootanchor (Variables|Default|GetShootAnchor))
  (bind _spawnedorb (Variables|Default|GetSpawnedOrb))
  (bind _returnvalue (Transformation|GetWorldTransform _shootanchor))
  ;[1 1 1] Shooting
  (:Pressed
    (Utilities|FlowControl|Sequence
      (:then_0
        ;;[1 1 1] Press Shoot
        (if (not (Variables|Default|GetHasOrbOut))
          (bind _returnvalue_2 (Effects|SpawnEmitterAttached "/Game/VFX_Toolkit_V1/ParticleSystems/356Days/Par_VoltCore_01.Par_VoltCore_01" _shootanchor "None" (.location _returnvalue) (Math|Rotator|MakeRotator (.roll (.rotation _returnvalue)) (+ (.pitch (.rotation _returnvalue)) 9e+01) (.yaw (.rotation _returnvalue))) "0.700000,0.700000,0.700000" "KeepWorldPosition" false))
          (Variables|Default|SetShootParticle _returnvalue_2)))))
  (:Released
    (Utilities|FlowControl|Sequence
      (:then_1
        ;;[1 1 1] Release Shoot
        (if (Variables|Default|GetHasOrbOut)
          (Utilities|FlowControl|DoOnce false :!label _label
            (:Completed
              (Variables|/Script/Engine.ProjectileMovementComponent|SetbSimulationEnabled (Variables|/Game/Blueprint/BP_EnergyOrb.BP_EnergyOrb_C|GetProjectileMovement _spawnedorb) false)
              (AI|RunBehaviorTree (AI|GetAIController _spawnedorb) "/Game/Blueprint/BT_EnergyOrb.BT_EnergyOrb")
              (Variables|Default|SetIsReturningOrb true)
              (Effects|SpawnEmitteratLocation "/Game/VFX_Toolkit_V1/ParticleSystems/356Days/Par_WildImpact_Purple.Par_WildImpact_Purple" (Transformation|GetWorldLocation (Variables|Default|GetShootAnchor)))
              (Effects|SpawnEmitteratLocation "/Game/VFX_Toolkit_V1/ParticleSystems/356Days/Par_WildImpact_Purple.Par_WildImpact_Purple" (Transformation|GetActorLocation (Variables|Default|GetSpawnedOrb)) "0, 0, 0" "3.000000,3.000000,3.000000")))
          (else
            (bind _shootparticle (Variables|Default|GetShootParticle)
              (:then
                (Components|DestroyComponent _shootparticle))
              (:else
                _))
            (CallFunction|ShootOrb)
            (goto _label Reset)))))))

(event Input|AxisEvents|InputAxisMoveForward
  (params (AxisValue :type Float%20%28single-precision%29))
  ;[1 1 1] Movement
  (Pawn|Input|AddMovementInput (Math|Vector|GetForwardVector (Math|Rotator|MakeRotator 0.0 0.0 (.yaw (Transformation|GetWorldRotation (Variables|Default|GetCamera))))) AxisValue false))

(event Input|AxisEvents|InputAxisMoveRight
  (params (AxisValue :type Float%20%28single-precision%29))
  ;[1 1 1] Movement
  (Pawn|Input|AddMovementInput (Math|Vector|GetRightVector (Math|Rotator|MakeRotator 0.0 0.0 (.yaw (Transformation|GetWorldRotation (Variables|Default|GetCamera))))) AxisValue false))

(event Input|AxisEvents|InputAxisMoveUp
  (params (AxisValue :type Float%20%28single-precision%29))
  ;[1 1 1] Movement
  (Pawn|Input|AddMovementInput (* (Math|Vector|GetUpVector (Math|Rotator|MakeRotator 0.0 0.0 (.yaw (Transformation|GetWorldRotation (Variables|Default|GetCamera))))) 2.0) AxisValue false))

(event Input|MouseEvents|MouseX
  (params (AxisValue :type Float%20%28single-precision%29))
  ;[1 1 1] Movement
  (Pawn|Input|AddControllerYawInput AxisValue))

(event Input|MouseEvents|MouseY
  (params (AxisValue :type Float%20%28single-precision%29))
  ;[1 1 1] Movement
  (Pawn|Input|AddControllerPitchInput (* AxisValue -1.0)))

(fn ConstructionScript)

(fn ShootOrb
  (bind _camera (Variables|Default|GetCamera))
  (bind _shootanchor (Variables|Default|GetShootAnchor))
  (bind _altanchor (Variables|Default|GetAltAnchor))
  (bind _returnvalue (Transformation|GetWorldLocation _camera))
  (bind _returnvalue_2 (Transformation|GetWorldLocation _shootanchor))
  (bind _returnvalue_3 (Transformation|GetWorldTransform _altanchor))
  (bind _returnvalue_4 (+ (.pitch (.rotation _returnvalue_3)) 9e+01))
  (bind _outhit (Collision|LineTraceByChannel _returnvalue (+ _returnvalue (* (Math|Vector|GetForwardVector _camera) 5e+03)) "TraceTypeQuery1" false 0 "None" true "(R=1.000000,G=0.000000,B=0.000000,A=1.000000)" "(R=0.000000,G=1.000000,B=0.000000,A=1.000000)" 1.0))
  (bind _output_get (Variables|Default|SetHitLoc (.traceend _outhit)))
  (bind _returnvalue_5 (Game|SpawnActorfromClass "/Game/Blueprint/BP_EnergyOrb.BP_EnergyOrb_C" (Math|Transform|MakeTransform _returnvalue_2 (Math|Rotator|FindLookatRotation _returnvalue_2 _output_get) "1.500000,1.500000,1.500000") "Undefined" 0 0))
  (Variables|Default|SetSpawnedOrb _returnvalue_5)
  (Variables|Default|SetHasOrbOut true)
  (Effects|SpawnEmitterAttached "/Game/VFX_Toolkit_V1/ParticleSystems/356Days/Par_FlashRing.Par_FlashRing" _altanchor "None" (.location _returnvalue_3) (Math|Rotator|MakeRotator (.roll (.rotation _returnvalue_3)) _returnvalue_4 (.yaw (.rotation _returnvalue_3))) "1.000000,1.000000,1.000000" "KeepWorldPosition")
  (Effects|SpawnEmitterAttached "/Game/FXVarietyPack/Particles/P_ky_hit1.P_ky_hit1" _altanchor "None" (.location _returnvalue_3) (Math|Rotator|MakeRotator (.roll (.rotation _returnvalue_3)) _returnvalue_4 (.yaw (.rotation _returnvalue_3))) "1.000000,1.000000,1.000000" "KeepWorldPosition")
  (Camera|PlayWorldCameraShake "/Game/Blueprint/BP_CamShake.BP_CamShake_C" (Transformation|GetWorldLocation (Variables|Collision|GetCapsuleComponent)) 0.0 1e+05 1.0 true))

(fn SetLerp
  (params (isEnterLerp :type Boolean) (TargetArmRot :type Rotator) (TargetCamRot :type Rotator))
  (Variables|Default|SetisEnterLerp isEnterLerp)
  (Variables|Default|SetCurArmRot (Variables|/Script/Engine.SceneComponent|GetRelativeRotation (Variables|Default|GetSpringArm)))
  (Variables|Default|SetCurCamRot (Variables|/Script/Engine.SceneComponent|GetRelativeRotation (Variables|Default|GetCamera)))
  (Variables|Default|SetTargetArmRot TargetArmRot)
  (Variables|Default|SetTargetCamRot TargetCamRot))